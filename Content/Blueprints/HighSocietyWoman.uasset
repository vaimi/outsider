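; High society woman NPC that plays an idle-state animation until told to run, then screams and switches to running.
; On BeginPlay it passes its TargetWaypoint to its RunAwayAIController, notifies it of the change and loops the default animation.
; The Run event activates the Scream component and loops the running animation directly on the mesh; it contains no movement logic.
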(event `Run`
  (`ActorComponent.Activate` (`self.Scream`) false)
  (`SkeletalMeshComponent.PlayAnimation` (`self.Mesh`) "/Game/Animations/HighSocietyRunning.HighSocietyRunning" true))

(event `self.ReceiveBeginPlay`
  (bind _asrun_away_aicontroller (cast `/Game/Blueprints/ExperimentalAI/RunAwayAIController` (`self.GetController`)))
  (set `/Game/Blueprints/ExperimentalAI/RunAwayAIController.TargetWaypoint` (`self.TargetWaypoint`) _asrun_away_aicontroller)
  (`/Game/Blueprints/ExperimentalAI/RunAwayAIController.TargetWaypointChanged` _asrun_away_aicontroller)
  (`SkeletalMeshComponent.PlayAnimation` (`self.Mesh`) "/Game/Animations/HighSociety_Anim.HighSociety_Anim" true))

(fn `UserConstructionScript`)