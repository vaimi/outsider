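; An AI controller for a run-away behavior that feeds waypoint and flee state to a behavior tree.
; On BeginPlay it resets the run-away flag, writes the target waypoint actor and location to the RunAway blackboard, then runs the RunAway behavior tree.
; The RunAwayTrigger event sets the run-away flag on the blackboard.
; TargetWaypointChanged rewrites the waypoint object and location keys.
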(event `RunAwayTrigger`
  (bind _output_get (set `self.RunAwayBool` true))
  (bind _blackboardcomponent (`self.UseBlackboard` "/Game/Blueprints/ExperimentalAI/RunAwayBlackboard.RunAwayBlackboard"))
  (`BlackboardComponent.SetValueAsBool` _blackboardcomponent (`self.RunAwayTriggered`) _output_get))

(event `self.ReceiveBeginPlay`
  (bind _targetwaypoint (`self.TargetWaypoint`))
  (bind _blackboardcomponent (`self.UseBlackboard` "/Game/Blueprints/ExperimentalAI/RunAwayBlackboard.RunAwayBlackboard"))
  (`BlackboardComponent.SetValueAsBool` _blackboardcomponent (`self.RunAwayTriggered`) false)
  (`BlackboardComponent.SetValueAsBool` _blackboardcomponent (`self.TrueBlackboardValue`) true)
  (`BlackboardComponent.SetValueAsObject` _blackboardcomponent (`self.TargetWaypointObject`) _targetwaypoint)
  (`BlackboardComponent.SetValueAsVector` _blackboardcomponent (`self.TargetWaypointLocation`) (`self.K2_GetActorLocation` _targetwaypoint))
  (`self.RunBehaviorTree` "/Game/Blueprints/ExperimentalAI/RunAwayBehavior.RunAwayBehavior"))

(event `TargetWaypointChanged`
  (bind _targetwaypoint (`self.TargetWaypoint`))
  (bind _blackboardcomponent (`self.UseBlackboard` "/Game/Blueprints/ExperimentalAI/RunAwayBlackboard.RunAwayBlackboard"))
  (`BlackboardComponent.SetValueAsObject` _blackboardcomponent (`self.TargetWaypointObject`) _targetwaypoint)
  (`BlackboardComponent.SetValueAsVector` _blackboardcomponent (`self.TargetWaypointLocation`) (`self.K2_GetActorLocation` _targetwaypoint)))

(fn `UserConstructionScript`)