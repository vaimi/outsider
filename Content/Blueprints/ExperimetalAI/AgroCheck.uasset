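; Behavior tree tick node that checks aggro for FollowerAIController pawns by finding nearby visible targets.
; Each tick, it sphere-traces for desired object types around the pawn, then line-traces to each hit on the Camera channel, ignoring SuperSoffa actors.
; Visible hits write TargetToFollow and TargetLocation to the blackboard; blocked hits clear only TargetToFollow.
; The loop never breaks, so the last hit decides the target.
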(event `self.ReceiveTickAI`
  (params (OwnerController :type "AIController Object Reference") (ControlledPawn :type "Pawn Object Reference") (DeltaSeconds :type "Float (single-precision)"))
  (bind _targettofollow (`self.TargetToFollow`))
  (bind _returnvalue (`Actor.K2_GetActorLocation` (`Controller.K2_GetPawn` (`self.AIControllerReference`))))
  (if (not (!= (`self.AIControllerReference`) null))
    (bind _asfollower_aicontroller (cast `/Game/Blueprints/ExperimetalAI/FollowerAIController` OwnerController))
    (set `self.AIControllerReference` _asfollower_aicontroller))
  (bind _outactors (`GameplayStatics.GetAllActorsOfClass` "/Game/Blueprints/ExperimetalAI/SuperSoffa.SuperSoffa_C"))
  (set `self.MyLocation` _returnvalue)
  (bind _outhits (`KismetSystemLibrary.SphereTraceMultiForObjects` _returnvalue (+ _returnvalue (0.0 0.0 15.0)) 1500.0 (`self.DesiredObjectTypes`) false _outactors))
  (for _array_element _outhits
    (bind (_bblockinghit _binitialoverlap _time _location _impactpoint _normal _impactnormal _physmat _hitactor) (`GameplayStatics.BreakHitResult` _array_element))
    (bind _outhit (`KismetSystemLibrary.LineTraceSingle` (`self.MyLocation`) (`Actor.K2_GetActorLocation` _hitactor) "TraceTypeQuery2" false _outactors))
    (bind (_bblockinghit_2 _binitialoverlap_2 _time_2 _location_2 _impactpoint_2 _normal_2 _impactnormal_2 _physmat_2 _hitactor_2) (`GameplayStatics.BreakHitResult` _outhit))
    (if (== _hitactor_2 _hitactor)
      (`BTFunctionLibrary.SetBlackboardValueAsObject` _targettofollow _hitactor_2)
      (`BTFunctionLibrary.SetBlackboardValueAsVector` (`self.TargetLocation`) (`Actor.K2_GetActorLocation` _hitactor_2))
      (else
        (`BTFunctionLibrary.SetBlackboardValueAsObject` _targettofollow)))))