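; CloseProximity is a behavior tree decorator for follower AI that, despite its name, passes when the pawn is at or beyond AcceptableDistance from its follow target.
; Its AI condition check casts the owning controller to FollowerAIController and stores the reference.
; It then reads the TargetToFollow actor from the blackboard and compares the straight-line distance between actor and pawn against that threshold.
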(fn `PerformConditionCheckAI`
  (params (OwnerController :type "AIController Object Reference") (ControlledPawn :type "Pawn Object Reference"))
  (returns (ReturnValue :type Boolean))
  (bind _asfollower_aicontroller (cast `/Game/Blueprints/ExperimetalAI/FollowerAIController` OwnerController))
  (set `self.AIControllerReference` _asfollower_aicontroller)
  (return (>= (`KismetMathLibrary.VSize` (- (`Actor.K2_GetActorLocation` (`BTFunctionLibrary.GetBlackboardValueAsActor` (`self.TargetToFollow`))) (`Actor.K2_GetActorLocation` ControlledPawn))) (`self.AcceptableDistance`))))